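; Combat component for the third-person player character that provides target lock and parry.
; The lock input toggles a target found by a debug-drawn pawn sphere trace ending ahead of the camera.
; While locked, Tick aims the control rotation at the target with a downward pitch offset and switches movement from orient-to-movement to controller-facing.
; Parry plays a samurai montage, gated by a flag until it completes or is interrupted.
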(event `self.ReceiveBeginPlay`
  (bind _charactermovement (`Character.CharacterMovement` (`self.Player BP`)))
  ;[1 1 1] Start  Movement Controller
  (bind _asbp_third_person_character (cast `/Game/ThirdPerson/Blueprints/BP_ThirdPersonCharacter` (`self.GetOwner`)))
  (set `self.Player BP` _asbp_third_person_character)
  (set `CharacterMovementComponent.bOrientRotationToMovement` true _charactermovement)
  (set `CharacterMovementComponent.bUseControllerDesiredRotation` false _charactermovement))

(event `EnhancedInput|/Game/ThirdPerson/Input/Actions/IA_Lock`
  (params (ActionValue :type Boolean) (ElapsedSeconds :type "Float (double-precision)") (TriggeredSeconds :type "Float (double-precision)") (InputAction :type "InputAction Object Reference" :default "/Game/ThirdPerson/Input/Actions/IA_Lock.IA_Lock"))
  (bind _transformcomponent (`PlayerCameraManager.TransformComponent` (`GameplayStatics.GetPlayerCameraManager` 0)))
  (bind _charactermovement (`Character.CharacterMovement` (`self.Player BP`)))
  (bind _charactermovement_2 (`Character.CharacterMovement` (`self.Player BP`)))
  (bind (_returnvalue_x _returnvalue_y _returnvalue_z) (`KismetMathLibrary.BreakVector` (`SceneComponent.K2_GetComponentLocation` _transformcomponent)))
  ;[1 1 1] Target Lock
  (:`Started`
    (if (`self.isTargetLock?`)
      (set `self.isTargetLock?` false)
      (set `self.Target Lock Actor` null)
      (set `CharacterMovementComponent.bOrientRotationToMovement` true _charactermovement_2)
      (set `CharacterMovementComponent.bUseControllerDesiredRotation` false _charactermovement_2)
      (else
        (`self.Target Lock Actor`
          (:`then`
            (set `self.Target Lock Actor` null)
            (set `CharacterMovementComponent.bOrientRotationToMovement` false _charactermovement)
            (set `CharacterMovementComponent.bUseControllerDesiredRotation` true _charactermovement))
          (:`else`
            (bind (_outhit _returnvalue) (`KismetSystemLibrary.SphereTraceSingleForObjects` :`End` (+ (`KismetMathLibrary.MakeVector` _returnvalue_x _returnvalue_y (+ _returnvalue_z 20.0)) (* (`KismetMathLibrary.GetForwardVector` (`SceneComponent.K2_GetComponentRotation` _transformcomponent)) 1000.0)) :`Radius` 150.0 :`ObjectTypes` (`|MakeArray` "ObjectTypeQuery3" :!type "EObjectTypeQuery Enum") :`DrawDebugType` "ForDuration" :`DrawTime` 2.0))
            (if _returnvalue
              (set `self.Target Lock Actor` (`.HitActor` (`GameplayStatics.BreakHitResult` _outhit)))
              (set `self.isTargetLock?` true)
              (else
                (set `self.isTargetLock?` false)))))))))

(event `self.ReceiveTick`
  (params (DeltaSeconds :type "Float (single-precision)"))
  (bind _charactermovement (`Character.CharacterMovement` (`self.Player BP`)))
  (bind (_returnvalue_roll _returnvalue_pitch _returnvalue_yaw) (`KismetMathLibrary.BreakRotator` (`KismetMathLibrary.FindLookAtRotation` (`Actor.K2_GetActorLocation` (`self.Player BP`)) (`Actor.K2_GetActorLocation` (`self.Target Lock Actor`)))))
  ;[1 1 1] Target Lock
  ;;[1 1 1] TargetLock
  (if (`self.isTargetLock?`)
    (`self.Target Lock Actor`
      (:`then`
        (`Controller.SetControlRotation` (`Pawn.GetController` (`self.Player BP`)) (`KismetMathLibrary.MakeRotator` _returnvalue_roll (+ _returnvalue_pitch -20.0) _returnvalue_yaw))
        (set `CharacterMovementComponent.bOrientRotationToMovement` false _charactermovement)
        (set `CharacterMovementComponent.bUseControllerDesiredRotation` true _charactermovement))
      (:`else`))))

(event `EnhancedInput|/Game/ThirdPerson/Input/Actions/IA_Parry`
  (params (ActionValue :type Boolean) (ElapsedSeconds :type "Float (double-precision)") (TriggeredSeconds :type "Float (double-precision)") (InputAction :type "InputAction Object Reference" :default "/Game/ThirdPerson/Input/Actions/IA_Parry.IA_Parry"))
  (:`Triggered`
    (if (not (`self.isParring?`))
      (set `self.isParring?` true)
      (`|PlayMontage` (`Character.Mesh` (`self.Player BP`)) "/Game/Characters/Souls/Parry/ARPG_Samurai_Anim_UE_Parry_Montage.ARPG_Samurai_Anim_UE_Parry_Montage"
        (:`OnCompleted`
          _)
        (:`OnInterrupted`
          _))
      (set `self.isParring?` false))))